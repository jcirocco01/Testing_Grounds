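; AI controller for a guard NPC that runs a behavior tree and fires on whatever actor it focuses.
; BeginPlay sets up the patrol blackboard and starts the tree.
; Perception stores a sensed player pawn as the enemy key, clearing it on lost sight or any non-player update.
; Tick drives the TP_Character's Aiming and Shoot flags from focus validity; FindPatrolRoute is an unfinished stub.
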(event `self.ReceiveTick`
  (params (DeltaSeconds :type "Float (single-precision)"))
  (bind _astp_character (cast `/Game/NPC/TP_Character` (`self.K2_GetPawn`)))
  (bind _output_get (set `/Game/NPC/TP_Character.Aiming` (`KismetSystemLibrary.IsValid` (`self.GetFocusActor`)) _astp_character))
  (set `/Game/NPC/TP_Character.Shoot` _output_get _astp_character))

(event `self.ReceiveBeginPlay`
  (bind _blackboardcomponent (`self.UseBlackboard` "/Game/NPC/BlackboardAssets/PatrolData.PatrolData"))
  (`self.RunBehaviorTree` "/Game/NPC/BlackboardAssets/GuardBehaviour.GuardBehaviour")
  (set `self.Blackboard Comp` _blackboardcomponent))

(event `self.AIPerception.OnTargetPerceptionUpdated`
  (params (Actor :type "Actor Object Reference") (Stimulus :type "AIStimulus Structure"))
  (if (`self.IsPlayerController` (`self.GetInstigatorController` Actor))
    (if (`.bSuccessfullySensed` (break `AIStimulus` Stimulus))
      (`BlackboardComponent.SetValueAsObject` (`self.Blackboard Comp`) (`self.EnemyKey`) Actor)
      (else
        (`BlackboardComponent.ClearValue` (`self.Blackboard Comp`) (`self.EnemyKey`) :!label _label)))
    (else
      (goto _label))))

(fn `Find Patrol Route`
  (params (BlackBoard :type "BlackboardComponent Object Reference")))

(fn `UserConstructionScript`)